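; BP_missile is a test homing missile actor that damages its assigned target on a hit.
; Initialize adds a scene component to the target and sets it as the ProjectileMovement homing target.
; For two seconds, Tick runs a short forward debug line trace, applying damage if it hits the target or printing a placeholder message otherwise.
; The missile destroys itself after any hit or when that time expires.
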(event Custom|homingStart
  (Variables|/Script/Engine.ProjectileMovementComponent|SetHomingTargetComponent (Variables|Default|GetProjectileMovement) (Variables|Default|GethomingTargetComp)))

(event Custom|initialize
  (params (target :type Actor%20Object%20Reference))
  (bind _output_get (Variables|Default|SetNewVar_0 target))
  (bind _returnvalue (AddComponent|AddSceneComponent _output_get false))
  (Variables|Default|SethomingTargetComp _returnvalue)
  (CallFunction|HomingStart))

(event Custom|destroy
  (Actor|DestroyActor))

(event EventBeginPlay)

(event Collision|EventActorBeginOverlap
  (params (OtherActor :type Actor%20Object%20Reference)))

(event EventTick
  (params (DeltaSeconds :type Float%20%28single-precision%29))
  (bind _returnvalue (Transformation|GetActorLocation))
  (bind _target (Variables|Default|Gettarget))
  (Variables|Default|Settime (+ (Variables|Default|Gettime) DeltaSeconds))
  (if (<= (Variables|Default|Gettime) 2.0)
    (bind (_outhit _returnvalue_2) (Collision|LineTraceByChannel _returnvalue (+ (* (Transformation|GetActorForwardVector) 1e+02) _returnvalue) "TraceTypeQuery1" false 0 "ForDuration"))
    (if _returnvalue_2
      (Utilities|FlowControl|DoOnce false
        (:Completed
          (if (== _target (.HitActor (Collision|BreakHitResult _outhit)))
            (Game|Damage|ApplyDamage _target 1e+02 0 0)
            (else
              (Development|PrintString "Hello")))
          (CallFunction|Destroy))))
    (else
      (Utilities|FlowControl|DoOnce false
        (:Completed
          (CallFunction|Destroy))))))

(fn ConstructionScript)

(fn SetHomingTarget
  (params (NewParam :type Actor%20Object%20Reference))
  (Variables|Default|SethomingTargetComp 0))