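; BP_Line is a test actor that builds and previews a clothoid curve through editable control points with start and end angles.
; The construction script uses SetParams2 to convert points to world space, passes them to CalcClothoidSpline, and debug-draws control and result points.
; BeginPlay feeds the cached results to UpdateSpline.
; The angle-converting SetParams, arrow drawing and turn-radius experiments are left disconnected.
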(event EventBeginPlay
  (Default|UpdateSpline (Variables|Default|GetNewVar_6) (Variables|Default|GetclothoidResults)))

(event Collision|EventActorBeginOverlap
  (params (OtherActor :type Actor%20Object%20Reference)))

(event EventTick
  (params (DeltaSeconds :type Float%20%28single-precision%29)))

(fn ConstructionScript
  ;[1 1 1] 準備
  (if (Variables|Default|GetNewVar_0)
    (Variables|Default|SetNewVar_0 false)
    (else
      (Variables|Default|SetNewVar_0 true)))
  (Utilities|Array|Clear (Variables|Default|Getpaths))
  (Utilities|Array|Clear (Variables|Default|GetclothoidPathParams))
  (if (> (Utilities|Array|Length (Variables|Default|Getbp_clothoidPathParams)) 1)
    (CallFunction|SetParams2)
    (Utilities|FlowControl|Sequence
      (:then_0
        (Development|PrintString "--------")
        (Utilities|FlowControl|Sequence
          (:then_0
            (for _array_element (Variables|Default|GetclothoidPathParams)
              (Rendering|Debug|DrawDebugPoint (.p_controll_loc _array_element) 25.0 "(R=1.000000,G=0.025771,B=0.085495,A=1.000000)" 1.0))
            ;[1 1 1] clothoid spline
            (bind _returnvalue (Class|ClothoidLine|CalcClothoidSpline (Variables|Default|GetclothoidPathParams)))
            (bind _output_get (Variables|Default|SetclothoidResults _returnvalue))
            (for _array_element_2 _output_get
              (Rendering|Debug|DrawDebugPoint _array_element_2 5.0 "(R=1.000000,G=0.000000,B=0.062831,A=1.000000)" (Variables|Default|GetclothoidLineDuration)))
            (Rendering|Debug|DrawDebugPoint (Variables|Default|Gettest_arcStartLoc) 1e+01 "(R=0.000000,G=0.000000,B=0.000000,A=1.000000)" (Variables|Default|GetclothoidLineDuration))))))))

(fn 新規関数0)

(fn DrawPathRotator
  (params (arrowSize :type Float%20%28single-precision%29) (duration :type Float%20%28single-precision%29) (thickness :type Float%20%28single-precision%29) (arrowLength :type Float%20%28single-precision%29))
  (LocalVariables|SetcolorCount 0)
  (for _index (range 0 (- (Utilities|Array|LastIndex (Variables|Default|Getbp_clothoidPathParams)) 1))
    (bind _output (CallFunction|GetColor (LocalVariables|GetarrowColors) (LocalVariables|GetcolorCount)))
    (LocalVariables|SetarrowColor _output)
    (Rendering|Debug|DrawDebugArrow (.p_controll_loc (Utilities|Array|Get(acopy) (Variables|Default|GetclothoidPathParams) (+ _index 1))) (+ (.p_controll_loc (Utilities|Array|Get(acopy) (Variables|Default|GetclothoidPathParams) (+ _index 1))) (* (Math|Vector|GetForwardVector (Math|Rotator|MakeRotator 0.0 0.0 (.phi1 (Utilities|Array|Get(acopy) (Variables|Default|GetclothoidPathParams) _index)))) arrowLength)) arrowSize (LocalVariables|GetarrowColor) duration thickness)
    (Rendering|Debug|DrawDebugArrow (.p_controll_loc (Utilities|Array|Get(acopy) (Variables|Default|GetclothoidPathParams) _index)) (+ (.p_controll_loc (Utilities|Array|Get(acopy) (Variables|Default|GetclothoidPathParams) _index)) (* (Math|Vector|GetForwardVector (Math|Rotator|MakeRotator 0.0 0.0 (.phi0 (Utilities|Array|Get(acopy) (Variables|Default|GetclothoidPathParams) _index)))) arrowLength)) arrowSize (LocalVariables|GetarrowColor) duration thickness))
  (return))

(fn GetClothoidphifromLocalphi
  (params (local_phi :type Float%20%28single-precision%29))
  (return (.yaw (Math|Rotator|Delta(Rotator) (Math|Rotator|MakeRotator 0.0 0.0 1.8e+02) (Math|Rotator|MakeRotator 0.0 0.0 local_phi)))))

(fn SetParams
  (bind _bp_clothoidpathparams (Variables|Default|Getbp_clothoidPathParams))
  (bind _returnvalue (Utilities|Array|LastIndex _bp_clothoidpathparams))
  (bind _output (Utilities|Array|Get(acopy) _bp_clothoidpathparams _returnvalue))
  (for _index (range 0 (- (Utilities|Array|LastIndex _bp_clothoidpathparams) 1))
    (LocalVariables|SetcurrentPathData (Utilities|Array|Get(acopy) _bp_clothoidpathparams _index))
    (LocalVariables|SetclothoidDegree (CallFunction|TransformClothoidDegree (Class|KismetMathLibrary|DegAtan2 (.y (- (.bp_p_loc (Utilities|Array|Get(acopy) _bp_clothoidpathparams (+ _index 1))) (.bp_p_loc (LocalVariables|GetcurrentPathData)))) (.x (- (.bp_p_loc (Utilities|Array|Get(acopy) _bp_clothoidpathparams (+ _index 1))) (.bp_p_loc (LocalVariables|GetcurrentPathData)))))))
    (Utilities|Array|Add (Variables|Default|GetclothoidPathParams) (Utilities|Struct|MakeClothoidPath (Math|Transform|TransformLocation (Transformation|GetActorTransform) (.bp_p_loc (LocalVariables|GetcurrentPathData))) (CallFunction|CalcPhi (.bp_phi1 (LocalVariables|GetcurrentPathData)) (LocalVariables|GetclothoidDegree)) (CallFunction|CalcPhi (.bp_phi0 (LocalVariables|GetcurrentPathData)) (LocalVariables|GetclothoidDegree))))
    (Development|PrintString (Utilities|String|ToString(Float) (LocalVariables|GetclothoidDegree))))
  (Utilities|Array|Add (Variables|Default|GetclothoidPathParams) (Utilities|Struct|MakeClothoidPath (Math|Transform|TransformLocation (Transformation|GetActorTransform) (.bp_p_loc _output)) (.bp_phi1 _output) (.bp_phi0 _output)))
  (return))

(fn GetColor
  (params (colors :type Array%20of%20Linear%20Color%20Structures) (index :type Integer%20%28by%20ref%29))
  (if (Utilities|Array|IsValidIndex colors index)
    (LocalVariables|Setresult (Utilities|Array|Get(acopy) colors index))
    (if (< (+ index 1) (Utilities|Array|Length colors))
      (Math|Integer|IncrementInt index
        (:%20%20
          _))
      (else
        (|SetBy-RefVar index)))
    (return (LocalVariables|Getresult))
    (else
      (return ""))))

(fn RangeFloat
  (params (input :type Float%20%28single-precision%29))
  (if (< input 1.8e+02)
    (if (>= input -1.8e+02)
      (return input)
      (else
        (return -1.8e+02)))
    (else
      (return 1.8e+02))))

(fn TransformClothoidDegree
  (params (input :type Float%20%28single-precision%29))
  (LocalVariables|SetlocalDegree input)
  (if (Math|Float|InRange(Float) (LocalVariables|GetlocalDegree) -1.8e+02 -9e+01)
    (return (- (Math|Float|Absolute(Float) (LocalVariables|GetlocalDegree)) 1.8e+02))
    (elif (Math|Float|InRange(Float) (LocalVariables|GetlocalDegree) -9e+01 0.0 false false)
      (return (- (Math|Float|Absolute(Float) (LocalVariables|GetlocalDegree)) 1.8e+02))
      (elif (Math|Float|InRange(Float) (LocalVariables|GetlocalDegree) 0.0 1.8e+02)
        (return (- 1.8e+02 (LocalVariables|GetlocalDegree)))
        (else
          (return 0.0))))))

(fn CombineFloat
  (params (input :type Float%20%28single-precision%29) (combineValue :type Float%20%28single-precision%29))
  (return (.yaw (Math|Rotator|CombineRotators (Math|Rotator|MakeRotator 0.0 0.0 input) (Math|Rotator|MakeRotator 0.0 0.0 combineValue)))))

(fn DeltaFloat
  (params (input :type Float%20%28single-precision%29) (deltaValue :type Float%20%28single-precision%29))
  (return (.yaw (Math|Rotator|Delta(Rotator) (Math|Rotator|MakeRotator 0.0 0.0 input) (Math|Rotator|MakeRotator 0.0 0.0 deltaValue)))))

(fn CalcPhi
  (params (curvature :type Float%20%28single-precision%29) (targetAngle :type Float%20%28single-precision%29))
  (LocalVariables|Setcurvature_inRange (CallFunction|RangeFloat curvature))
  (if (Math|Float|InRange(Float) targetAngle 0.0 1.8e+02 false)
    (return (* (- (+ (LocalVariables|Getcurvature_inRange) targetAngle) 1.8e+02) -1.0))
    (elif (Math|Float|InRange(Float) targetAngle -1.8e+02 0.0)
      (return (* (+ (+ (LocalVariables|Getcurvature_inRange) targetAngle) 1.8e+02) -1.0))
      (else
        (Development|PrintString (Utilities|String|Append "ERROR : TargetAngle " (Utilities|String|ToString(Float) targetAngle)))
        (return 0.0)))))

(fn SetParams2
  (for _array_element (Variables|Default|Getbp_clothoidPathParams)
    (Utilities|Array|Add (Variables|Default|GetclothoidPathParams) (Utilities|Struct|MakeClothoidPath (Math|Transform|TransformLocation (Transformation|GetActorTransform) (.bp_p_loc _array_element)) (.bp_phi1 _array_element) (.bp_phi0 _array_element))))
  (return))