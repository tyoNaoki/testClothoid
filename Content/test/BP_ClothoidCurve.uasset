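; Test actor that previews clothoid curves as debug points.
; The construction script builds a triple clothoid from PointMark to the local-space Target with start and end angles Phi0 and Phi1, when their XY distance exceeds one unit, and draws it briefly.
; Curve math comes from functions defined outside this graph; local helpers cover single-segment drawing, curvature and index ranges.
; Disconnected experiments remain, including multi-curve and chained-actor variants; the Draw branch has no effect.
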(event EventBeginPlay)

(event Collision|EventActorBeginOverlap
  (params (OtherActor :type Actor%20Object%20Reference)))

(event EventTick
  (params (DeltaSeconds :type Float%20%28single-precision%29)))

(fn ConstructionScript
  (bind _returnvalue (Transformation|GetActorTransform))
  (bind _pointmark (Variables|Default|GetpointMark))
  (bind _target (Variables|Parametor|Gettarget))
  (bind _returnvalue_2 (Transformation|GetWorldLocation _pointmark))
  (bind _returnvalue_3 (Math|Transform|TransformLocation _returnvalue _target))
  (if (Variables|Default|Getdraw)
    _
    (else
      _))
  (Variables|Default|Setdraw false)
  (if (> (CallFunction|CalcR _returnvalue_3 _returnvalue_2) 1.0)
    (bind _returnvalue_4 (Class|ClothoidLine|TripleClothoidCurve (Variables|Default|GetcheckTripleParam) (Variables|Parametor|Getphi1) (Variables|Parametor|Getphi0) _returnvalue_2 _returnvalue_3))
    (for (_array_element _array_index) _returnvalue_4
      (Rendering|Debug|DrawDebugPoint _array_element 1e+01 "(R=1.000000,G=0.000000,B=0.000000,A=1.000000)" 2.0))))

(fn OnClothoidCurve
  (params (PointColor :type Linear%20Color%20Structure))
  (bind _h (Variables|Parametor|Geth))
  (if (<= (Math|Conversions|ToFloat(Integer) (Variables|Parametor|Getnum)) _h)
    _
    (else
      (Variables|Parametor|Setnum (Math|Float|Truncate _h))))
  (bind _returnvalue (Class|ClothoidLine|ClothoidCurve (Variables|Parametor|Getnum) _h (Variables|Parametor|Getphi0) (Variables|Parametor|GetphiV) (Variables|Parametor|GetphiU) (Transformation|GetWorldLocation (Variables|Default|GetpointMark))))
  (for _array_element _returnvalue
    (Rendering|Debug|DrawDebugPoint _array_element 5.0 PointColor 2.0))
  (return _returnvalue))

(fn CalcPhiV
  (params (phiV :type Float%20%28single-precision%29))
  (bind _s (LocalVariables|Gets))
  (return (Math|Trig|RadiansToDegrees (+ (* (Math|Trig|DegreesToRadians phiV) _s) (* (Math|Trig|DegreesToRadians (Variables|Parametor|GetphiU)) (Math|Float|Power _s 2.0))))))

(fn CalcR
  (params (H :type Float%20%28single-precision%29) (s :type Float%20%28single-precision%29) (phiV :type Float%20%28single-precision%29) (phiU :type Float%20%28single-precision%29))
  (bind _returnvalue (* phiU 2.0))
  (bind _returnvalue_2 (* _returnvalue s))
  (bind _returnvalue_3 (+ phiV _returnvalue_2))
  (if (and (> H 0.0) (> _returnvalue_3 0.0))
    (return (/ _returnvalue_3 H))
    (else
      (return 0.0))))

(fn CalcR
  (params (lastLoc :type Vector) (startLoc :type Vector))
  (return (Math|Vector|VectorLengthXY (- lastLoc startLoc))))

(fn InRangeLine
  (params (index :type Integer) (length :type Integer) (range :type Float%20%28single-precision%29))
  (return (< index (Math|Float|Truncate (* length range)))))

(fn IsRangeLine
  (params (index :type Integer) (length :type Integer) (range :type Float%20%28single-precision%29))
  (return (== index (Math|Float|Truncate (* length range)))))