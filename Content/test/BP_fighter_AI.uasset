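; AI fighter aircraft that flies a spline path and detects other BP_fighter actors as lock-on targets.
; Each tick it advances by distance along the path, banking from the interpolated yaw difference to a look-ahead point, and stops near the end.
; A forward sphere trace, filtered by an angle comparison and line-of-sight trace, refreshes LockOnTargets.
; Clothoid waypoint and turn-radius experiments remain unconnected.
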(event Custom|flyingAnimation
  (params (InputPin :type Float%20%28single-precision%29))
  (bind _newvar_0 (Variables|Default|GetNewVar_0))
  (bind _newvar_0_2 (Variables|Default|GetNewVar_0))
  (if (not (Variables|Default|Getstop))
    (Utilities|IsValid _newvar_0_2
      (:Is%20Valid
        (if (Variables|/Game/test/BP_Spline.BP_Spline_C|Getinitiaze _newvar_0_2)
          (Variables|Default|SetmoveDis (+ (Variables|Default|GetmoveDis) (* InputPin (Variables|Default|GetmoveSpeed))))
          (bind _newparam (Default|GetCurrentLocation _newvar_0 true (Variables|Default|GetmoveDis)))
          (bind _returnvalue (Default|GetRotation _newvar_0))
          (bind _returnvalue_2 (Default|GetNextRotation _newvar_0 1e+02))
          (Transformation|SetActorLocationAndRotation _newparam (Math|Rotator|MakeRotator (Math|Interpolation|FInterpTo (Variables|Default|GetcurrentYaw) (.yaw (Math|Rotator|Delta(Rotator) (Math|Rotator|MakeRotator 0.0 0.0 (.yaw _returnvalue_2)) (Math|Rotator|MakeRotator 0.0 0.0 (.yaw _returnvalue)))) (Utilities|Time|GetWorldDeltaSeconds) 1.0) (.pitch _returnvalue) (.yaw _returnvalue)))
          (Variables|Default|SetcurrentYaw (Math|Interpolation|FInterpTo (Variables|Default|GetcurrentYaw) (.yaw (Math|Rotator|Delta(Rotator) (Math|Rotator|MakeRotator 0.0 0.0 (.yaw _returnvalue_2)) (Math|Rotator|MakeRotator 0.0 0.0 (.yaw _returnvalue)))) (Utilities|Time|GetWorldDeltaSeconds) 1.0))
          (if (<= (Math|Float|Absolute(Float) (- (Spline|GetSplineLength (Variables|/Game/test/BP_Spline.BP_Spline_C|GetSpline (Variables|Default|GetNewVar_0))) (Variables|Default|GetmoveDis))) 1e+02)
            (Variables|Default|Setstop true)))))))

(event EventBeginPlay)

(event Collision|EventActorBeginOverlap
  (params (OtherActor :type Actor%20Object%20Reference)))

(event EventTick
  (params (DeltaSeconds :type Float%20%28single-precision%29))
  (CallFunction|FlyingAnimation DeltaSeconds)
  (Variables|Default|SetlockOnStartPosi (+ (Transformation|GetWorldLocation (Variables|Default|GetfirePosition)) (* (Math|Vector|GetForwardVector (Transformation|GetActorRotation)) (Variables|Default|GetlockonStartDistace))))
  (bind (_outhits _returnvalue) (Collision|MultiSphereTraceByChannel (Variables|Default|GetlockOnStartPosi) (+ (* (Math|Vector|GetForwardVector (Transformation|GetActorRotation)) (Variables|Default|GetlockonDistance)) (Variables|Default|GetlockOnStartPosi)) 5e+02 "TraceTypeQuery1" false 0 "None"))
  (if _returnvalue
    (Utilities|FlowControl|DoOnce false :!label _label
      (:Completed
        (Utilities|Array|Clear (Variables|Default|GetlocallockOnTarget))
        (bind _array_element (Utilities|Array|ForEachLoopwithBreak _outhits)
          (:LoopBody
            (bind _asbp_fighter (Utilities|Casting|CastToBP_fighter (.HitActor (Collision|BreakHitResult _array_element))))
            (if (< (Variables|Default|GetsightAngle) (CallFunction|GetAngletoTarget _asbp_fighter))
              (bind _outhit (Collision|LineTraceByChannel (Transformation|GetWorldLocation (Variables|Default|GetfirePosition)) (Transformation|GetActorLocation (.HitActor (Collision|BreakHitResult _array_element))) "TraceTypeQuery1" false 0 "None"))
              (if (== (.HitActor (Collision|BreakHitResult _array_element)) (.HitActor (Collision|BreakHitResult _outhit)))
                (Utilities|Array|Add (Variables|Default|GetlocallockOnTarget) _asbp_fighter))))
          (:Completed
            (Utilities|FlowControl|Sequence
              (:then_0
                (Variables|Default|SetlockOnTargets (Variables|Default|GetlocallockOnTarget)))
              (:then_1
                (goto _label Reset)))))))))

(fn ConstructionScript
  (bind _staticmesh (Variables|Default|GetStaticMesh))
  (bind _returnvalue (Transformation|GetWorldRotation _staticmesh))
  (Transformation|SetWorldRotation _staticmesh (Math|Rotator|MakeRotator (.roll _returnvalue) (Variables|Default|Getpitch) (.yaw _returnvalue)) false false))

(fn FindRoute)

(fn CalcRadius
  (params (V :type Float%20%28single-precision%29) (theta :type Float%20%28single-precision%29))
  (LocalVariables|Setspeed (/ (* (* V 1.852) 1e+03) 3.6e+03))
  (LocalVariables|SetbankAngle (* theta (/ (Math|Trig|GetPI) 1.8e+02)))
  (return (/ (Math|Float|Square (LocalVariables|Getspeed)) (* 9.8 (Math|Trig|Tan(Radians) (LocalVariables|GetbankAngle))))))

(fn GetAngletoTarget
  (params (target :type Actor%20Object%20Reference))
  (bind _returnvalue (Transformation|GetActorLocation target))
  (bind _returnvalue_2 (Transformation|GetActorLocation))
  (bind _returnvalue_3 (Transformation|GetActorForwardVector))
  (bind _returnvalue_4 (- _returnvalue _returnvalue_2))
  (return (Class|KismetMathLibrary|DegAcos (/ (Math|Vector|DotProduct _returnvalue_3 _returnvalue_4) (* (Math|Vector|VectorLength _returnvalue_3) (Math|Vector|VectorLength _returnvalue_4))))))