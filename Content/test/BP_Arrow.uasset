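; Test actor that visualizes an aircraft-style banked turn at the corner of a three-point path, entirely in the construction script.
; It converts Input points to world space and derives turn radius from speed in knots and bank angle.
; The circle's center sits along the corner's angle bisector, and Arrow points tangent at an offset start point, signed by turn direction.
; Results are debug-drawn and printed; clothoid helpers and other experiments remain unconnected.
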(event EventBeginPlay)

(event Collision|EventActorBeginOverlap
  (params (OtherActor :type Actor%20Object%20Reference)))

(event EventTick
  (params (DeltaSeconds :type Float%20%28single-precision%29)))

(fn ConstructionScript
  (bind _paths (Variables|Default|Getpaths))
  (bind _v (Variables|Default|GetV))
  (bind _theta (Variables|Default|Gettheta))
  (bind _scale (Variables|Default|Getscale))
  (bind _paths_2 (Variables|Default|Getpaths))
  (bind _turningradius (CallFunction|CalculateTurningRadius _v _theta _scale))
  (bind _output (Utilities|Array|Get(acopy) _paths 1))
  (bind _output_2 (Utilities|Array|Get(acopy) _paths_2))
  (bind _output_3 (Utilities|Array|Get(acopy) _paths_2 1))
  (bind _output_4 (Utilities|Array|Get(acopy) _paths_2 2))
  (bind _returnvalue (Math|Rotator|FindLookatRotation _output_3 _output_4))
  (bind _returnvalue_2 (Math|Rotator|FindLookatRotation _output_3 _output_2))
  (bind _returnvalue_3 (CallFunction|GetThreePointAngle _output_2 _output_3 _output_4))
  (bind _returnvalue_4 (CallFunction|GetMiddleAngle (.yaw _returnvalue_2) (.yaw _returnvalue)))
  (bind _returnvalue_5 (Math|Rotator|MakeRotator 0.0 0.0 _returnvalue_4))
  (bind _returnvalue_6 (Math|Vector|GetForwardVector _returnvalue_5))
  (bind _returnvalue_7 (* _returnvalue_6 _turningradius))
  (bind _returnvalue_8 (+ _returnvalue_7 _output_3))
  (Utilities|Array|Clear (Variables|Default|Getpaths))
  (for _array_element (Variables|Default|Getinput)
    (Utilities|Array|Add (Variables|Default|Getpaths) (Math|Transform|TransformLocation (Transformation|GetActorTransform) _array_element)))
  (if (Utilities|Array|IsValidIndex _paths_2 2)
    (LocalVariables|SetthreeP_Angle _returnvalue_3)
    (Development|PrintString (Utilities|String|ToString(Float) _returnvalue_3))
    (Rendering|Debug|DrawDebugCircle _returnvalue_8 _turningradius 30 "(R=1.000000,G=0.000000,B=0.102115,A=1.000000)" 5.0 5.0 "0.000000,1.000000,0.000000" "1.000000,0.000000,0.000000")
    (Development|PrintString (Utilities|String|Append "Radius : " (Utilities|String|ToString(Float) _turningradius)))
    (Rendering|Debug|DrawDebugPoint (CallFunction|GetAngleLocOfCircle (.yaw (Math|Rotator|Delta(Rotator) (Math|Rotator|CombineRotators _returnvalue_5 "0,180.000000, 0") (Math|Rotator|MakeRotator 0.0 0.0 (* (Math|Float|Sign(Float) (LocalVariables|GetthreeP_Angle)) (Variables|Default|GetcircleStartAngle))))) _turningradius _returnvalue_8) 3e+01 "(R=0.327070,G=1.000000,B=0.000000,A=1.000000)" 5.0)
    (Development|PrintString (Utilities|String|Append "rot : " (Utilities|String|ToString(Float) 0.0)))
    (Rendering|Debug|DrawDebugArrow (+ (CallFunction|GetAngleLocOfCircle (.yaw (Math|Rotator|Delta(Rotator) (Math|Rotator|CombineRotators _returnvalue_5 "0,180.000000, 0") (Math|Rotator|MakeRotator 0.0 0.0 (* (Math|Float|Sign(Float) (LocalVariables|GetthreeP_Angle)) (Variables|Default|GetcircleStartAngle))))) _turningradius _returnvalue_8) (* "0, 0, 0" 1e+02)) (+ (CallFunction|GetAngleLocOfCircle (.yaw (Math|Rotator|Delta(Rotator) (Math|Rotator|CombineRotators _returnvalue_5 "0,180.000000, 0") (Math|Rotator|MakeRotator 0.0 0.0 (* (Math|Float|Sign(Float) (LocalVariables|GetthreeP_Angle)) (Variables|Default|GetcircleStartAngle))))) _turningradius _returnvalue_8) "0, 0, 0") 5.0 "(R=0.015724,G=0.087294,B=1.000000,A=1.000000)" 5.0 1e+01)
    (Transformation|SetWorldRotation (Variables|Default|GetArrow) (Math|Rotator|CombineRotators (Math|Rotator|FindLookatRotation _returnvalue_8 (CallFunction|GetAngleLocOfCircle (.yaw (Math|Rotator|Delta(Rotator) (Math|Rotator|CombineRotators _returnvalue_5 "0,180.000000, 0") (Math|Rotator|MakeRotator 0.0 0.0 (* (Math|Float|Sign(Float) (LocalVariables|GetthreeP_Angle)) (Variables|Default|GetcircleStartAngle))))) _turningradius _returnvalue_8)) (Math|Rotator|MakeRotator 0.0 0.0 (* (Math|Float|Sign(Float) (.Z (Math|Vector|BreakVector (Math|Vector|CrossProduct (- (Utilities|Array|Get(acopy) _paths) _output) (- _output (Utilities|Array|Get(acopy) _paths 2)))))) 9e+01))) false false)))

(fn TransformClothoidDegree
  (params (input :type Float%20%28single-precision%29))
  (if (Math|Float|InRange(Float) input -1.8e+02 -9e+01)
    (return (- (Math|Float|Absolute(Float) input) 1.8e+02))
    (elif (Math|Float|InRange(Float) input -9e+01 0.0 false false)
      (return (- (Math|Float|Absolute(Float) input) 1.8e+02))
      (elif (Math|Float|InRange(Float) input 0.0 1.8e+02 false false)
        (return (- 1.8e+02 input))
        (else
          (return 0.0))))))

(fn CombineFloat
  (params (input :type Float%20%28single-precision%29) (combineValue :type Float%20%28single-precision%29))
  (return (.yaw (Math|Rotator|CombineRotators (Math|Rotator|MakeRotator 0.0 0.0 input) (Math|Rotator|MakeRotator 0.0 0.0 combineValue)))))

(fn DeltaFlaot
  (params (input :type Float%20%28single-precision%29) (deltaValue :type Float%20%28single-precision%29))
  (return (.yaw (Math|Rotator|Delta(Rotator) (Math|Rotator|MakeRotator 0.0 0.0 input) (Math|Rotator|MakeRotator 0.0 0.0 deltaValue)))))

(fn CalculateTurningRadius
  (params (v :type Float%20%28single-precision%29) (theta :type Float%20%28single-precision%29) (scale :type Float%20%28single-precision%29))
  (LocalVariables|Setspeed (/ (* (* v 1.852) 1e+03) 3.6e+03))
  (LocalVariables|SetbankAngle (* theta (/ (Math|Trig|GetPI) 1.8e+02)))
  (return (/ (/ (Math|Float|Square (LocalVariables|Getspeed)) (* 9.8 (Math|Trig|Tan(Radians) (LocalVariables|GetbankAngle)))) scale)))

(fn CalcCircle
  (params (arcRadius :type Float%20%28single-precision%29) (NewParam :type Vector))
  (Rendering|Debug|DrawDebugCircle NewParam arcRadius 30 "(R=0.109160,G=1.000000,B=0.123469,A=1.000000)" 2.0 2.0 "0.000000,1.000000,0.000000" "1.000000,0.000000,0.000000"))

(fn CalculateTurningRadiusM/s
  (params (v :type Float%20%28single-precision%29) (theta :type Float%20%28single-precision%29))
  (return (/ (Math|Float|Square v) (* 9.8 (Math|Trig|Tan(Degrees) theta)))))

(fn SpeedtoKt
  (params (speed :type Float%20%28single-precision%29))
  (return (/ speed 5.0)))

(fn CalcT
  (params (bank_angle :type Float%20%28single-precision%29))
  (LocalVariables|Setspeed 514.0)
  (bind _output_get (LocalVariables|SetturnningRad 3e+01))
  (Development|PrintString (Utilities|String|Append "Rad : " (Utilities|String|ToString(Float) _output_get)))
  (return (/ (* (* 2.0 (Math|Trig|GetPI)) (LocalVariables|GetturnningRad)) (Math|Float|Sqrt (* (LocalVariables|GetturnningRad) 9.8)))))

(fn DrawCircle
  (params (startAngle :type Float%20%28single-precision%29) (endAngle :type Float%20%28single-precision%29) (radius :type Float%20%28single-precision%29) (centerLocation :type Vector))
  (bind _returnvalue (Math|Float|Truncate startAngle))
  (bind _returnvalue_2 (Math|Float|Truncate endAngle))
  (for _index (range (Math|Float|Truncate startAngle) (Math|Float|Truncate endAngle))
    (Rendering|Debug|DrawDebugPoint (+ centerLocation (Math|Vector|MakeVector (* radius (Math|Trig|Cos(Degrees) (Math|Conversions|ToFloat(Integer) _index))) (* radius (Math|Trig|Sin(Degrees) (Math|Conversions|ToFloat(Integer) _index))) 0.0)) 1e+01 "(R=1.000000,G=0.808993,B=0.000000,A=1.000000)" 1.0))
  (LocalVariables|SetstartLoc (+ (Transformation|GetActorLocation) (Math|Vector|MakeVector (* radius (Math|Trig|Cos(Degrees) (Math|Conversions|ToFloat(Integer) _returnvalue))) (* radius (Math|Trig|Sin(Degrees) (Math|Conversions|ToFloat(Integer) _returnvalue))) 0.0)))
  (LocalVariables|SetendLoc (+ (Transformation|GetActorLocation) (Math|Vector|MakeVector (* radius (Math|Trig|Cos(Degrees) (Math|Conversions|ToFloat(Integer) _returnvalue_2))) (* radius (Math|Trig|Sin(Degrees) (Math|Conversions|ToFloat(Integer) _returnvalue_2))) 0.0)))
  (return (LocalVariables|GetstartLoc) (LocalVariables|GetendLoc)))

(fn CalcStartAngle
  (params (r :type Float%20%28single-precision%29) (a :type Float%20%28single-precision%29))
  (LocalVariables|SetL (/ (Math|Float|Square a) r))
  (return (Math|Trig|Tan(Degrees) (/ (LocalVariables|GetL) (* a 2.0)))))

(fn GetThreePointAngle
  (params (A :type Vector) (B :type Vector) (A2 :type Vector))
  (bind _returnvalue (- A B))
  (bind _returnvalue_2 (- B A2))
  (bind _returnvalue_3 (Math|Vector|CrossProduct _returnvalue _returnvalue_2))
  (return (* (Class|KismetMathLibrary|DegAtan2 (Math|Vector|VectorLength _returnvalue_3) (Math|Vector|DotProduct _returnvalue _returnvalue_2)) (Math|Float|Sign(Float) (.Z (Math|Vector|BreakVector _returnvalue_3))))))

(fn GetMiddleAngle
  (params (a1 :type Float%20%28single-precision%29) (a2 :type Float%20%28single-precision%29))
  (bind _returnvalue (Math|Trig|DegreesToRadians a1))
  (bind _returnvalue_2 (Math|Trig|DegreesToRadians a2))
  (LocalVariables|Setx1 (Math|Trig|Cos(Radians) _returnvalue))
  (LocalVariables|Sety1 (Math|Trig|Sin(Radians) _returnvalue))
  (LocalVariables|Setx2 (Math|Trig|Cos(Radians) _returnvalue_2))
  (LocalVariables|Sety2 (Math|Trig|Sin(Radians) _returnvalue_2))
  (LocalVariables|Setx (/ (+ (LocalVariables|Getx1) (LocalVariables|Getx2)) 2.0))
  (LocalVariables|Sety (/ (+ (LocalVariables|Gety1) (LocalVariables|Gety2)) 2.0))
  (return (Class|KismetMathLibrary|DegAtan2 (LocalVariables|Gety) (LocalVariables|Getx))))

(fn GetAngleLocOfCircle
  (params (angle :type Float%20%28single-precision%29) (radius :type Float%20%28single-precision%29) (centerLocation :type Vector))
  (LocalVariables|SetcirLoc (+ centerLocation (Math|Vector|MakeVector (* radius (Math|Trig|Cos(Degrees) angle)) (* radius (Math|Trig|Sin(Degrees) angle)) 0.0)))
  (return (LocalVariables|GetcirLoc)))