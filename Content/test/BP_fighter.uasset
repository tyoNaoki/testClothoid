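; Test fighter actor that flies along a path supplied by NewVar0, advancing its travelled distance by MoveSpeed each Tick.
; It takes pitch and yaw from the path, easing roll toward the yaw difference from a look-ahead rotation to bank into turns.
; Construction sets mesh pitch and prints a turn radius computed by CalcRadius from knots and bank angle.
; Older BpLine clothoid-following and circling code is disconnected, and FindRoute is empty.
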(event EventBeginPlay)

(event Collision|EventActorBeginOverlap
  (params (OtherActor :type Actor%20Object%20Reference)))

(event EventTick
  (params (DeltaSeconds :type Float%20%28single-precision%29))
  (bind _newvar_0 (Variables|Default|GetNewVar_0))
  (if (Variables|/Game/test/BP_Spline.BP_Spline_C|Getinitiaze (Variables|Default|GetNewVar_0))
    (Variables|Default|SetmoveDis (+ (Variables|Default|GetmoveDis) (* DeltaSeconds (Variables|Default|GetmoveSpeed))))
    (bind _newparam (Default|GetCurrentLocation _newvar_0 true (Variables|Default|GetmoveDis)))
    (bind _returnvalue (Default|GetRotation _newvar_0))
    (bind _returnvalue_2 (Default|GetNextRotation _newvar_0 1e+02))
    (Transformation|SetActorLocationAndRotation _newparam (Math|Rotator|MakeRotator (Math|Interpolation|FInterpTo (Variables|Default|GetcurrentYaw) (.yaw (Math|Rotator|Delta(Rotator) (Math|Rotator|MakeRotator 0.0 0.0 (.yaw _returnvalue_2)) (Math|Rotator|MakeRotator 0.0 0.0 (.yaw _returnvalue)))) (Utilities|Time|GetWorldDeltaSeconds) 1.0) (.pitch _returnvalue) (.yaw _returnvalue)))
    (Variables|Default|SetcurrentYaw (Math|Interpolation|FInterpTo (Variables|Default|GetcurrentYaw) (.yaw (Math|Rotator|Delta(Rotator) (Math|Rotator|MakeRotator 0.0 0.0 (.yaw _returnvalue_2)) (Math|Rotator|MakeRotator 0.0 0.0 (.yaw _returnvalue)))) (Utilities|Time|GetWorldDeltaSeconds) 1.0))))

(fn ConstructionScript
  (bind _staticmesh (Variables|Default|GetStaticMesh))
  (bind _returnvalue (Transformation|GetWorldRotation _staticmesh))
  (Transformation|SetWorldRotation _staticmesh (Math|Rotator|MakeRotator (.roll _returnvalue) (Variables|Default|Getpitch) (.yaw _returnvalue)) false false)
  (Development|PrintString (Utilities|String|ToString(Float) (/ (CallFunction|CalcRadius (Variables|Default|GetmoveSpeed) (Variables|Default|Getpitch)) 1e+01))))

(fn FindRoute)

(fn CalcRadius
  (params (V :type Float%20%28single-precision%29) (theta :type Float%20%28single-precision%29))
  (LocalVariables|Setspeed (/ (* (* V 1.852) 1e+03) 3.6e+03))
  (LocalVariables|SetbankAngle (* theta (/ (Math|Trig|GetPI) 1.8e+02)))
  (return (/ (Math|Float|Square (LocalVariables|Getspeed)) (* 9.8 (Math|Trig|Tan(Radians) (LocalVariables|GetbankAngle))))))